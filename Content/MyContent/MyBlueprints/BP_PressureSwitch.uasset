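; BP_PressureSwitch is a pressure switch actor that activates a linked door while a qualifying object rests on it.
; Its Box overlap events only respond to actors implementing BPI_SwitchObjTrigger.
; Begin overlap swaps the Button to an emissive material instance and calls SwitchActivated on DoorToActivate; end overlap restores the base material and calls SwitchDeactivated, without counting overlapping objects.
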(event OnComponentBeginOverlap(Box)
  (params (OverlappedComponent :type Primitive%20Component%20Object%20Reference) (OtherActor :type Actor%20Object%20Reference) (OtherComp :type Primitive%20Component%20Object%20Reference) (OtherBodyIndex :type Integer) (bFromSweep :type Boolean) (SweepResult :type Hit%20Result%20Structure%20%28by%20ref%29))
  (if (Utilities|DoesObjectImplementInterface OtherActor "/Game/MyContent/MyBlueprints/BPI_SwitchObjTrigger.BPI_SwitchObjTrigger_C")
    (Rendering|Material|CreateDynamicMaterialInstance (Variables|Default|GetButton) 0 "/Game/MyContent/MyMaterials/MI_Emmisive.MI_Emmisive" "None" :!class /Script/Engine.PrimitiveComponent)
    (Default|SwitchActivated (Variables|Default|GetDoorToActivate))))

(event OnComponentEndOverlap(Box)
  (params (OverlappedComponent :type Primitive%20Component%20Object%20Reference) (OtherActor :type Actor%20Object%20Reference) (OtherComp :type Primitive%20Component%20Object%20Reference) (OtherBodyIndex :type Integer))
  (if (Utilities|DoesObjectImplementInterface OtherActor "/Game/MyContent/MyBlueprints/BPI_SwitchObjTrigger.BPI_SwitchObjTrigger_C")
    (Rendering|Material|CreateDynamicMaterialInstance (Variables|Default|GetButton) 0 "/Game/MyContent/MyMaterials/M_Emmisive.M_Emmisive" "None" :!class /Script/Engine.PrimitiveComponent)
    (Default|SwitchDeactivated (Variables|Default|GetDoorToActivate))))

(fn ConstructionScript)