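; BP_Door is an interactable door that stays locked until enough keys are collected and switches are active.
; Key and switch events update their counters and re-evaluate the lock, which is also checked on BeginPlay.
; When unlocked, Interact uses a FlipFlop to play or reverse a timeline that lerps the door's yaw.
; Two overlap volumes toggle an interact prompt widget and a locked widget, the latter shown only while requirements are unmet.
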(event OnComponentBeginOverlap(DoorLocked)
  (params (OverlappedComponent :type Primitive%20Component%20Object%20Reference) (OtherActor :type Actor%20Object%20Reference) (OtherComp :type Primitive%20Component%20Object%20Reference) (OtherBodyIndex :type Integer) (bFromSweep :type Boolean) (SweepResult :type Hit%20Result%20Structure%20%28by%20ref%29))
  (bind _lockedwidget (Variables|Default|GetLockedWidget))
  ;[0.15 0.15 0.15 0.5] Widget Pop Up Logic
  (if (and (>= (Variables|Default|GetKeysCollected) (Variables|Default|GetRequiredKeyAmount)) (>= (Variables|Default|GetSwitchesActive) (Variables|Default|GetRequiredSwitches)))
    (Rendering|SetVisibility _lockedwidget false false)
    (else
      (Rendering|SetVisibility _lockedwidget true false))))

(event OnComponentEndOverlap(DoorLocked)
  (params (OverlappedComponent :type Primitive%20Component%20Object%20Reference) (OtherActor :type Actor%20Object%20Reference) (OtherComp :type Primitive%20Component%20Object%20Reference) (OtherBodyIndex :type Integer))
  ;[0.15 0.15 0.15 0.5] Widget Pop Up Logic
  (Rendering|SetVisibility (Variables|Default|GetLockedWidget) false false))

(event OnComponentBeginOverlap(WidgetPopUp)
  (params (OverlappedComponent :type Primitive%20Component%20Object%20Reference) (OtherActor :type Actor%20Object%20Reference) (OtherComp :type Primitive%20Component%20Object%20Reference) (OtherBodyIndex :type Integer) (bFromSweep :type Boolean) (SweepResult :type Hit%20Result%20Structure%20%28by%20ref%29))
  ;[0.15 0.15 0.15 0.5] Widget Pop Up Logic
  (Rendering|SetVisibility (Variables|Components|GetEWidget) true false))

(event OnComponentEndOverlap(WidgetPopUp)
  (params (OverlappedComponent :type Primitive%20Component%20Object%20Reference) (OtherActor :type Actor%20Object%20Reference) (OtherComp :type Primitive%20Component%20Object%20Reference) (OtherBodyIndex :type Integer))
  ;[0.15 0.15 0.15 0.5] Widget Pop Up Logic
  (Rendering|SetVisibility (Variables|Components|GetEWidget) false false))

(event Custom|SwitchActivated
  ;[0.15 0.15 0.15 0.5] Switch Activation/ Deactivation
  (Math|Integer|IncrementInt (Variables|Default|GetSwitchesActive)
    (:%20%20
      (CallFunction|CheckDoorStatus))))

(event Custom|SwitchDeactivated
  ;[0.15 0.15 0.15 0.5] Switch Activation/ Deactivation
  (Math|Integer|DecrementInt (Variables|Default|GetSwitchesActive)
    (:%20%20
      (CallFunction|CheckDoorStatus))))

(event Custom|CheckDoorStatus
  ;[0.15 0.15 0.15 0.5] Checks if Door is Locked
  (Variables|Default|SetLocked (not (and (>= (Variables|Default|GetKeysCollected) (Variables|Default|GetRequiredKeyAmount)) (>= (Variables|Default|GetSwitchesActive) (Variables|Default|GetRequiredSwitches))))))

(event EventInteract
  ;[0.15 0.15 0.15 0.5] How Door Opens
  (if (not (Variables|Default|GetLocked))
    (Utilities|FlowControl|FlipFlop
      (:A
        (bind _doorroatation (Timeline|OpenDoorTimeline Play)
          (:Update
            (Transformation|SetRelativeRotation (Variables|Components|GetDoor) (Math|Rotator|MakeRotator 0.0 0.0 (Math|Float|Lerp 0.0 1.1e+02 _doorroatation)) false false))))
      (:B
        (Timeline|OpenDoorTimeline Reverse)))))

(event EventIncrementKeysCollected
  ;[0.15 0.15 0.15 0.5] How Keys are Incremented
  (Math|Integer|IncrementInt (Variables|Default|GetKeysCollected)
    (:%20%20
      (CallFunction|CheckDoorStatus))))

(event EventBeginPlay
  (CallFunction|CheckDoorStatus))

(fn ConstructionScript)